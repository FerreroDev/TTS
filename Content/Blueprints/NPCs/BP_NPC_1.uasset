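; BP_NPC_1 is an NPC Blueprint that the player can take control of through a Possess event.
; The event prints a debug message and blends the player camera to the NPC over a short time.
; After a delay matching the blend, the first player controller possesses the NPC and input is enabled on it.
; The construction script only calls the parent version.
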(event EventPossess
  ;[1 1 1] Being Possessed
  (Development|PrintString "I was possessed")
  (Game|Player|SetViewTargetwithBlend (Game|GetPlayerController 0) self 1.0 "VTBlend_Linear" 0.0 false)
  (Utilities|FlowControl|Delay 1.0)
  (Pawn|Possess (Game|GetPlayerController 0) self)
  (Input|EnableInput self (Game|GetPlayerController 0)))

(fn ConstructionScript
  (|CallParentFunction))